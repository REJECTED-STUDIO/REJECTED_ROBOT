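; BP_BasicPlatform is a moving platform that cycles its static mesh through an array of target locations.
; On BeginPlay, if CanMove is set, it moves the mesh to the current relative location over MoveDuration with MoveComponentTo, then waits WaitDuration.
; It then advances the index, wrapping to the first entry after the last, and calls MovePlatform again to loop.
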(event `self.ReceiveBeginPlay`
  (`self.MovePlatform`))

(event `MovePlatform`
  (bind _returnvalue (+ (`self.VectorIndex`) 1))
  (if (`self.CanMove`)
    (`KismetSystemLibrary.MoveComponentTo` (`self.StaticMesh`) (`|GetArrayItem` (`self.TargetLocation`) (`self.VectorIndex`)) (struct) false false (`self.MoveDuration`))
    (`KismetSystemLibrary.Delay` (`self.WaitDuration`))
    (set `self.VectorIndex` (select `bool` (<= _returnvalue (`KismetArrayLibrary.Array_LastIndex` (`self.TargetLocation`))) :`true` _returnvalue))
    (`self.MovePlatform`)))

(fn `UserConstructionScript`)
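; BP_Light is a light actor in the world-manipulation system that switches on at night and off by day.
; Night and day interface notifications each start a timeline that drives the point light's intensity up to a scaled maximum.
; A TurnedOn flag and DoOnce gates, reset when each timeline finishes, stop repeated notifications from restarting a fade.
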(event `/Game/BPInterfaces/BPI_WorldManipulation.BPI_NotifyNight`
  (if (not (`self.TurnedOn`))
    (`/Engine/EditorBlueprintResources/StandardMacros.DoOnce` false :!label _label
      (:`Completed`
        (bind (_direction _newtrack_2) (`Timeline|TurnOn` :!via `PlayFromStart`)
          (:`Update`
            (`LightComponent.SetIntensity` (`self.PointLight`) (* _newtrack_2 5000.0)))
          (:`Finished`
            (set `self.TurnedOn` true)
            (goto _label :!via `Reset`)))))))

(event `/Game/BPInterfaces/BPI_WorldManipulation.BPI_NotifyDay`
  (if (`self.TurnedOn`)
    (`/Engine/EditorBlueprintResources/StandardMacros.DoOnce` false :!label _label_2
      (:`Completed`
        (bind (_direction _newtrack_2) (`Timeline|Timeline` :!via `PlayFromStart`)
          (:`Update`
            (`LightComponent.SetIntensity` (`self.PointLight`) (* _newtrack_2 5000.0)))
          (:`Finished`
            (set `self.TurnedOn` false)
            (goto _label_2 :!via `Reset`)))))))

(fn `UserConstructionScript`)
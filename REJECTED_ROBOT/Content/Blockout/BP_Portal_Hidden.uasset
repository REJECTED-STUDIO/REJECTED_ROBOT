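; Blockout portal actor that can start hidden and teleports overlapping actors to a linked portal once it is opened.
; On BeginPlay the Widze variable sets whether the static mesh is hidden in game.
; The BPIOpenPortal event reveals the mesh and enables the Teleport flag.
; While that flag is set, any actor that begins overlapping the mesh moves to the location and rotation of the referenced portal's Target.
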(event `self.ReceiveBeginPlay`
  (`SceneComponent.SetHiddenInGame` (`self.StaticMesh`) (`self.Widze`) false))

(event `self.StaticMesh.OnComponentBeginOverlap`
  (params (OverlappedComponent :type "PrimitiveComponent Object Reference") (OtherActor :type "Actor Object Reference") (OtherComp :type "PrimitiveComponent Object Reference") (OtherBodyIndex :type Integer) (bFromSweep :type Boolean) (SweepResult :type "HitResult Structure (by ref)"))
  (bind (_returnvalue_location _returnvalue_rotation) (`KismetMathLibrary.BreakTransform` (`SceneComponent.K2_GetComponentToWorld` (`/Game/Blockout/BP_Portal_Hidden.Target` (`self.bp_portal`)))))
  (if (`self.Teleport`)
    (`self.K2_TeleportTo` OtherActor _returnvalue_location _returnvalue_rotation)))

(event `/Game/BPInterfaces/BPI_ItemsInteractive.BPI_OpenPortal`
  (`SceneComponent.SetHiddenInGame` (`self.StaticMesh`) false false)
  (set `self.Teleport` true))

(fn `UserConstructionScript`)
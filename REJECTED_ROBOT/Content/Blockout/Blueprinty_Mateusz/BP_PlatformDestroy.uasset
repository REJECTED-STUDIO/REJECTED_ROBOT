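; Blockout platform actor that disappears some time after its mesh is hit and later comes back.
; The mesh hit event waits DeathTime, calls CantTouch, waits ReviveTime, then calls it again.
; CantTouch sets actor collision and in-game visibility from the ActoriExist flag, then flips it, so one event handles both vanishing and restoring.
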(event `self.StaticMesh.OnComponentHit`
  (params (HitComponent :type "PrimitiveComponent Object Reference") (OtherActor :type "Actor Object Reference") (OtherComp :type "PrimitiveComponent Object Reference") (NormalImpulse :type "Vector Structure") (Hit :type "HitResult Structure (by ref)"))
  (`KismetSystemLibrary.Delay` (`self.DeathTime`))
  (`self.CantTouch`)
  (`KismetSystemLibrary.Delay` (`self.ReviveTime`))
  (`self.CantTouch`))

(event `CantTouch`
  (`self.SetActorEnableCollision` self (`self.ActoriExist?`))
  (`self.SetActorHiddenInGame` self (not (`self.ActoriExist?`)))
  (set `self.ActoriExist?` (not (`self.ActoriExist?`))))

(fn `UserConstructionScript`)
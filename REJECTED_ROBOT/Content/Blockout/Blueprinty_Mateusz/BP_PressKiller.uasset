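; BP_PressKiller is a crushing press hazard that cycles back and forth and kills what it touches.
; From BeginPlay, KillArea moves the Press component to LocationEnd and back to LocationStart with separately timed MoveComponentTo moves, waits, then calls itself to loop forever.
; Overlapping the Box sends BPIPlayerDeathMessage to the other actor through an interface call, with no check on the press's position or actor type.
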(event `self.ReceiveBeginPlay`
  (`self.KillArea`))

(event `KillArea`
  (bind _press (`self.Press`))
  (`KismetSystemLibrary.MoveComponentTo` _press (`self.Location_End`) (struct) false false (`self.TimeToKill`))
  (`KismetSystemLibrary.MoveComponentTo` _press (`self.Location_Start`) (struct) false false (`self.TimeGo`))
  (`KismetSystemLibrary.Delay` (`self.TimeToWait`))
  (`self.KillArea`))

(event `self.Box.OnComponentBeginOverlap`
  (params (OverlappedComponent :type "PrimitiveComponent Object Reference") (OtherActor :type "Actor Object Reference") (OtherComp :type "PrimitiveComponent Object Reference") (OtherBodyIndex :type Integer) (bFromSweep :type Boolean) (SweepResult :type "HitResult Structure (by ref)"))
  (message `/Game/BPInterfaces/BPI_PlayerInteraction.BPI_PlayerDeath` OtherActor))

(fn `UserConstructionScript`)
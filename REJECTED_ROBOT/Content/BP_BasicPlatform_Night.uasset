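; Platform that exists only at night, fading in and turning solid on the night notification, then fading out and losing collision on the day one.
; Collision and CanMove switch half a second after each fade starts, and night also calls MovePlatform.
; Two timelines drive the material Opacity parameter, gated by DoOnce nodes that each reset when the opposite fade finishes, so fades alternate.
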(event `self.ReceiveBeginPlay`)

(event `/Game/BPInterfaces/BPI_WorldManipulation.BPI_NotifyNight`
  (`self.FadeIn`)
  (`KismetSystemLibrary.Delay` 0.5)
  (`PrimitiveComponent.SetCollisionEnabled` (`self.StaticMesh`) "QueryAndPhysics")
  (set `self.CanMove` true)
  (`self.MovePlatform`))

(event `/Game/BPInterfaces/BPI_WorldManipulation.BPI_NotifyDay`
  (`self.FadeOut`)
  (`KismetSystemLibrary.Delay` 0.5)
  (`PrimitiveComponent.SetCollisionEnabled` (`self.StaticMesh`) "NoCollision")
  (set `self.CanMove` false))

(event `FadeIn`
  (`/Engine/EditorBlueprintResources/StandardMacros.DoOnce` false :!label _label
    (:`Completed`
      (bind (_direction _fadein_out) (`Timeline|Timeline` :!via `PlayFromStart`)
        (:`Update`
          (`MeshComponent.SetScalarParameterValueOnMaterials` (`self.StaticMesh`) "Opacity" (`KismetMathLibrary.Lerp` 0.0 1.0 _fadein_out)))
        (:`Finished`
          (goto _label_2 :!via `Reset`))))))

(event `FadeOut`
  (`/Engine/EditorBlueprintResources/StandardMacros.DoOnce` false :!label _label_2
    (:`Completed`
      (bind (_direction _fadein_out) (`Timeline|Timeline_0` :!via `PlayFromStart`)
        (:`Update`
          (`MeshComponent.SetScalarParameterValueOnMaterials` (`self.StaticMesh`) "Opacity" (`KismetMathLibrary.Lerp` 0.0 1.0 _fadein_out)))
        (:`Finished`
          (goto _label :!via `Reset`))))))

(fn `UserConstructionScript`
  (`parent.UserConstructionScript`))
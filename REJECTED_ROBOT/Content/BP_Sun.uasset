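; BP_Sun is a sun actor that toggles the world between day and night on a debug F key press.
; A FlipFlop alternately notifies all BPI_WorldManipulation actors of night or day, then plays or reverses a Timeline.
; The Timeline lerps the actor's relative rotation through 180 degrees, and the IsSet flag blocks a new transition until the current one finishes.
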(event EventBeginPlay
  (Input|EnableInput (Game|GetPlayerController 0)))

(event Input|KeyboardEvents|DebugKeyF
  (params (Key :type Key%20Structure :default "None") (ActionValue :type Input%20Action%20Value%20Structure))
  (:Pressed
    (Utilities|FlowControl|FlipFlop
      (:A
        (if (Variables|Default|GetIsSet)
          (bind _outactors (Actor|GetAllActorswithInterface "/Game/BPInterfaces/BPI_WorldManipulation.BPI_WorldManipulation_C"))
          (Class|BPIWorldManipulation|BPINotifyNight(Message) _outactors)
          (Variables|Default|SetIsSet false)
          (bind _y (Timeline|Timeline Play)
            (:Update
              (Transformation|SetActorRelativeRotation (Math|Rotator|Lerp(Rotator) "0, 0, 0" "180.000000,0.000000,0.000000" _y)))
            (:Finished
              (Variables|Default|SetIsSet true)))))
      (:B
        (if (Variables|Default|GetIsSet)
          (bind _outactors_2 (Actor|GetAllActorswithInterface "/Game/BPInterfaces/BPI_WorldManipulation.BPI_WorldManipulation_C"))
          (Class|BPIWorldManipulation|BPINotifyDay(Message) _outactors_2)
          (Variables|Default|SetIsSet false)
          (Timeline|Timeline Reverse))))))

(fn ConstructionScript)
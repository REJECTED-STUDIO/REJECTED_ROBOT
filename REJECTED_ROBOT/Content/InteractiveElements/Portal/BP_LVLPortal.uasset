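; BP_LVLPortal is a portal actor that opens another level when the player character overlaps its static mesh.
; An interface event sets the Level index, updates the text render with the matching name from ListaNazw, and swaps the mesh to that destination's portal material.
; On overlap, the same index selects which map to open, such as the hub or tutorial.
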(event `self.StaticMesh.OnComponentBeginOverlap`
  (params (OverlappedComponent :type "PrimitiveComponent Object Reference") (OtherActor :type "Actor Object Reference") (OtherComp :type "PrimitiveComponent Object Reference") (OtherBodyIndex :type Integer) (bFromSweep :type Boolean) (SweepResult :type "HitResult Structure (by ref)"))
  (if (== OtherActor (`GameplayStatics.GetPlayerCharacter` 0))
    (`GameplayStatics.OpenLevelBySoftObjectPtr` (select `int` (stale `/Game/BPInterfaces/BPI_PlayerInteraction.BPI_SetLevelToOpen` _output_get) :`0` "/Game/Game_Ready_Levels/M_HUB.M_HUB" :`1` "/Game/Game_Ready_Levels/LVL_Tutorial.LVL_Tutorial" :`2` "/Game/Game_Ready_Levels/Zagadki_01.Zagadki_01" :`3` "/Game/Game_Ready_Levels/Level_Gabriel_1.Level_Gabriel_1" :`4` "/Game/Game_Ready_Levels/Proba.Proba" :!type "World Soft Object Reference"))))

(event `/Game/BPInterfaces/BPI_PlayerInteraction.BPI_SetLevelToOpen`
  (params (Level :type Integer))
  (bind _staticmesh (`self.StaticMesh`))
  (bind _output_get (set `self.Level` Level))
  (`TextRenderComponent.K2_SetText` (`self.TextRender`) (`KismetTextLibrary.Conv_StringToText` (`KismetStringLibrary.Conv_NameToString` (`|GetArrayItem` (`self.ListaNazw`) (`self.Level`)))))
  (switch `int` (`self.Level`)
    (:`Default`
      (`PrimitiveComponent.SetMaterial` _staticmesh 0 "/Game/Materials_Made/Portal/MI_Portal01.MI_Portal01" :!label _label))
    (:`0`
      (goto _label))
    (:`1`
      (`PrimitiveComponent.SetMaterial` _staticmesh 0 "/Game/Materials_Made/Portal/MI_Portal02.MI_Portal02"))
    (:`2`
      (`PrimitiveComponent.SetMaterial` _staticmesh 0 "/Game/Materials_Made/Portal/MI_Portal03.MI_Portal03"))
    (:`3`
      (`PrimitiveComponent.SetMaterial` _staticmesh 0 "/Game/Materials_Made/Portal/MI_Portal04.MI_Portal04"))
    (:`4`
      (`PrimitiveComponent.SetMaterial` _staticmesh 0 "/Game/Materials_Made/Portal/MI_Portal05.MI_Portal05"))))

(fn `UserConstructionScript`)
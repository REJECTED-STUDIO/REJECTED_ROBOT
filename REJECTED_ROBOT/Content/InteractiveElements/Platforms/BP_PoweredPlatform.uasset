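; Moving platform that runs only while powered, switched on and off through interaction interface events.
; The parent's BeginPlay runs only if IsPowered is already true at start.
; The call and dismiss interaction events set or clear IsPowered, then CheckIfPowered either calls MovePlatform or stops MovingTimeline.
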(event `self.ReceiveBeginPlay`
  (if (`self.IsPowered`)
    (`parent.ReceiveBeginPlay`)))

(event `/Game/BPInterfaces/BPI_PlayerInteraction.BPI_CallInteraction`
  (set `self.IsPowered` true)
  (`self.CheckIfPowered` :!label _label))

(event `/Game/BPInterfaces/BPI_PlayerInteraction.BPI_DismissInteraction`
  (set `self.IsPowered` false)
  (goto _label))

(event `CheckIfPowered`
  (if (`self.IsPowered`)
    (`self.MovePlatform`)
    (else
      (`TimelineComponent.Stop` (`self.MovingTimeline`)))))

(fn `UserConstructionScript`
  (`parent.UserConstructionScript`))
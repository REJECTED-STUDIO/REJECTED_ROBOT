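; BP_BasicPlatform is a moving platform that cycles its mesh endlessly through a list of relative target locations from BeginPlay.
; MovingTimeline lerps from the mesh's current location toward the indexed target, so the start point shifts every update.
; On finish it advances or wraps the index, waits, then replays and resets the timeline.
; MoveSpeed sets play rate at construction; an older MoveComponentTo path is disconnected.
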(event `self.ReceiveBeginPlay`
  (`self.MovePlatform`))

(event `MovePlatform`
  (bind _returnvalue (+ (`self.VectorIndex`) 1))
  (bind (_direction _newtrack_0) (`Timeline|MovingTimeline` :!label _label)
    (:`Update`
      (`SceneComponent.K2_SetRelativeLocation` (`self.StaticMesh`) (`KismetMathLibrary.VLerp` (`SceneComponent.RelativeLocation` (`self.StaticMesh`)) (`|GetArrayItem` (`self.TargetLocation`) (`self.VectorIndex`)) _newtrack_0) false false))
    (:`Finished`
      (set `self.VectorIndex` (select `bool` (<= _returnvalue (`KismetArrayLibrary.Array_LastIndex` (`self.TargetLocation`))) :`true` _returnvalue))
      (`KismetSystemLibrary.Delay` (`self.WaitDuration`))
      (`self.MovePlatform`)
      (goto _label :!via `SetNewTime`))))

(fn `UserConstructionScript`
  (`TimelineComponent.SetPlayRate` (`self.MovingTimeline`) (`self.MoveSpeed`)))
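; Moving platform actor that travels continuously through a looping list of points from BeginPlay.
; MoveToPoint uses a latent MoveComponentTo to move the Platform component to the current Points entry as a relative location, taking GoTime per move.
; It then increments the index, wraps to zero past the end, and calls itself again.
; An unconnected SetActorLocation to the first point never runs.
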(event `self.ReceiveBeginPlay`
  (`self.MoveToPoint`))

(event `MoveToPoint`
  (`KismetSystemLibrary.MoveComponentTo` (`self.Platform`) (`|GetArrayItem` (`self.Points`) (`self.NumberOfPoin`)) (struct) false false (`self.GoTime`))
  (bind _result (`/Engine/EditorBlueprintResources/StandardMacros.IncrementInt` (`self.NumberOfPoin`))
    (:`  `
      (set `self.NumberOfPoin` _result)
      (if (<= (`KismetArrayLibrary.Array_Length` (`self.Points`)) (`self.NumberOfPoin`))
        (set `self.NumberOfPoin` 0)
        (`self.MoveToPoint`)
        (else
          (`self.MoveToPoint`))))))

(fn `UserConstructionScript`)
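; Night variant of a basic moving platform that becomes lethal to touch at night.
; Night notification starts a material opacity timeline that sets Killer and, after a short delay, enables movement.
; Day notification stops movement and runs a second timeline with another material that clears Killer, with paired DoOnce gates alternating the fades.
; Mesh hits while Killer is set send a player death interface message to the other actor.
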(event `self.ReceiveBeginPlay`)

(event `self.BPI_NotifyNight`
  (`self.FadeIn`)
  (`KismetSystemLibrary.Delay` 0.5)
  (set `self.CanMove` true)
  (`self.MovePlatform`))

(event `self.BPI_NotifyDay`
  (`self.FadeOut`)
  (`KismetSystemLibrary.Delay` 0.5)
  (set `self.CanMove` false))

(event `FadeIn`
  (`/Engine/EditorBlueprintResources/StandardMacros.DoOnce` false :!label _label
    (:`Completed`
      (`PrimitiveComponent.SetMaterial` (`self.StaticMesh`) 0 "/Game/InteractiveElements/Platforms/NightPlatform/M_FadeIN-OUT.M_FadeIN-OUT")
      (bind (_direction _fadein_out) (`Timeline|Timeline` :!via `PlayFromStart`)
        (:`Update`
          (`MeshComponent.SetScalarParameterValueOnMaterials` (`self.StaticMesh`) "Opacity" (`KismetMathLibrary.Lerp` 0.0 1.0 _fadein_out))
          (set `self.Killer?` true))
        (:`Finished`
          (goto _label_2 :!via `Reset`))))))

(event `FadeOut`
  (`/Engine/EditorBlueprintResources/StandardMacros.DoOnce` false :!label _label_2
    (:`Completed`
      (`PrimitiveComponent.SetMaterial` (`self.StaticMesh`) 0 "/Game/Nell/Materials/M_Mushroom_02.M_Mushroom_02")
      (bind (_direction _fadein_out) (`Timeline|Timeline_0` :!via `PlayFromStart`)
        (:`Update`
          (`MeshComponent.SetScalarParameterValueOnMaterials` (`self.StaticMesh`) "Opacity" (`KismetMathLibrary.Lerp` 0.0 1.0 _fadein_out))
          (set `self.Killer?` false))
        (:`Finished`
          (goto _label :!via `Reset`))))))

(event `self.StaticMesh.OnComponentHit`
  (params (HitComponent :type "PrimitiveComponent Object Reference") (OtherActor :type "Actor Object Reference") (OtherComp :type "PrimitiveComponent Object Reference") (NormalImpulse :type "Vector Structure") (Hit :type "HitResult Structure (by ref)"))
  (if (`self.Killer?`)
    (message `/Game/BPInterfaces/BPI_PlayerInteraction.BPI_PlayerDeath` OtherActor)))

(fn `UserConstructionScript`
  (`parent.UserConstructionScript`))
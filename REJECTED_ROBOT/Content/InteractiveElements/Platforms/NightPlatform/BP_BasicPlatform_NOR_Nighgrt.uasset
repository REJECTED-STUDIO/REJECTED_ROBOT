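; Platform Blueprint variant that reacts to day and night notifications, being solid by day and non-colliding at night.
; Each notification swaps the mesh material at once, then after a short delay toggles collision and the CanMove flag.
; Night clears CanMove and calls MovePlatform, while day only sets the flag.
; BeginPlay is empty, with the parent call disabled, so the parent's startup logic does not run.
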(event `self.ReceiveBeginPlay`)

(event `self.BPI_NotifyNight`
  (`PrimitiveComponent.SetMaterial` (`self.StaticMesh`) 0 "/Game/Blockout/Assets/Materials/M_White.M_White")
  (`KismetSystemLibrary.Delay` 0.5)
  (`PrimitiveComponent.SetCollisionEnabled` (`self.StaticMesh`) "NoCollision")
  (set `self.CanMove` false)
  (`self.MovePlatform`))

(event `self.BPI_NotifyDay`
  (`PrimitiveComponent.SetMaterial` (`self.StaticMesh`) 0 "/Game/InteractiveElements/Platforms/NightPlatform/M_FadeIN-OUT.M_FadeIN-OUT")
  (`KismetSystemLibrary.Delay` 0.5)
  (`PrimitiveComponent.SetCollisionEnabled` (`self.StaticMesh`) "QueryAndPhysics")
  (set `self.CanMove` true))

(fn `UserConstructionScript`
  (`parent.UserConstructionScript`))
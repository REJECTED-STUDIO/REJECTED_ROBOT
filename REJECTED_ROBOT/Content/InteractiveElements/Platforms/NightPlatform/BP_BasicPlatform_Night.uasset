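; BP_BasicPlatform_Night is a moving platform variant that is active only at night.
; Night and day notifications each wait half a second, then toggle the mesh collision and the CanMove flag.
; Night also calls MovePlatform to start movement, while day only disables collision and clears the flag.
; BeginPlay does nothing, as its parent call is disabled, so activation depends on those notifications.
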(event `self.ReceiveBeginPlay`)

(event `/Game/BPInterfaces/BPI_WorldManipulation.BPI_NotifyNight`
  (`KismetSystemLibrary.Delay` 0.5)
  (`PrimitiveComponent.SetCollisionEnabled` (`self.StaticMesh`) "QueryAndPhysics")
  (set `self.CanMove` true)
  (`self.MovePlatform`))

(event `/Game/BPInterfaces/BPI_WorldManipulation.BPI_NotifyDay`
  (`KismetSystemLibrary.Delay` 0.5)
  (`PrimitiveComponent.SetCollisionEnabled` (`self.StaticMesh`) "NoCollision")
  (set `self.CanMove` false))

(fn `UserConstructionScript`
  (`parent.UserConstructionScript`))
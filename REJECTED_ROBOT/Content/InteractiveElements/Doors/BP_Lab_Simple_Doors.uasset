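; BP_Lab_Simple_Doors is an interactive lab door that slides open and closed.
; The construction script applies the configurable door mesh, and BeginPlay stores the mesh's starting relative location.
; The interface interaction call plays a timeline that lerps the mesh from that base location to a target location.
; Dismissing the interaction reverses the timeline to slide it back.
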(event `self.ReceiveBeginPlay`
  (set `self.BaseLocation` (`SceneComponent.RelativeLocation` (`self.StaticMesh`))))

(event `self.BPI_CallInteraction`
  (bind (_direction _ot) (`Timeline|OpeningTimeline` :`NewTime` (`self.TimeToMove`) :!label _label)
    (:`Update`
      (`SceneComponent.K2_SetRelativeLocation` (`self.StaticMesh`) (`KismetMathLibrary.VLerp` (`self.BaseLocation`) (`self.TargetLocation`) _ot) false false))))

(event `self.BPI_DismissInteraction`
  (goto _label :!via `Reverse`))

(fn `UserConstructionScript`
  (`StaticMeshComponent.SetStaticMesh` (`self.StaticMesh`) (`self.DoorsMesh`)))
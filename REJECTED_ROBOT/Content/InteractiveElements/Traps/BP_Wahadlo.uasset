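; Pendulum trap (Wahadlo) that swings continuously and kills what it touches.
; From BeginPlay, a FlipFlop alternates playing a timeline forward and in reverse, re-triggering after a short delay whenever it finishes.
; The timeline lerps the mesh's relative rotation from zero to Rotation, with Speed setting its play rate in the construction script.
; Capsule overlaps send BPIPlayerDeathMessage to the other actor without filtering.
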(event `self.ReceiveBeginPlay`
  (`self.Attack`))

(event `Attack`
  (`/Engine/EditorBlueprintResources/StandardMacros.FlipFlop` :!label _label
    (:`A`
      (bind (_direction _newtrack_0) (`Timeline|Timeline` :!via `PlayFromStart` :!label _label_2)
        (:`Update`
          (`SceneComponent.K2_SetRelativeRotation` (`self.StaticMesh`) (`KismetMathLibrary.RLerp` (struct) (`self.Rotation`) _newtrack_0) false false))
        (:`Finished`
          (`KismetSystemLibrary.Delay` 0.2)
          (goto _label))))
    (:`B`
      (goto _label_2 :!via `Reverse`))))

(event `self.Capsule.OnComponentBeginOverlap`
  (params (OverlappedComponent :type "PrimitiveComponent Object Reference") (OtherActor :type "Actor Object Reference") (OtherComp :type "PrimitiveComponent Object Reference") (OtherBodyIndex :type Integer) (bFromSweep :type Boolean) (SweepResult :type "HitResult Structure (by ref)"))
  (message `/Game/BPInterfaces/BPI_PlayerInteraction.BPI_PlayerDeath` OtherActor))

(fn `UserConstructionScript`
  (`TimelineComponent.SetPlayRate` (`self.Timeline`) (`self.Speed`)))
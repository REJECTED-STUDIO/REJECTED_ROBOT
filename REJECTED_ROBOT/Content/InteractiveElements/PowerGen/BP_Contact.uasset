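; BP_Contact is a power-generation contact element that shows its powered state and passes it on to a target cable.
; Its connected and disconnected interface events behave identically, switching the static mesh between powered and powerless materials based on the Power flag.
; It then sends the cable an interaction call when powered or a dismiss message when not, through interface messages.
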(event `/Game/BPInterfaces/BPI_PowerSystem.BPI_IsConnected`
  (params (Power :type Boolean))
  (bind _staticmesh (`self.StaticMesh`))
  (bind _targetcable (`self.TargetCable`))
  (if Power
    (`PrimitiveComponent.SetMaterial` _staticmesh 0 "/Game/InteractiveElements/PowerGen/M_Power.M_Power")
    (message `/Game/BPInterfaces/BPI_PlayerInteraction.BPI_CallInteraction` _targetcable :!label _label)
    (else
      (`PrimitiveComponent.SetMaterial` _staticmesh 0 "/Game/InteractiveElements/PowerGen/M_Powerless.M_Powerless")
      (message `/Game/BPInterfaces/BPI_PlayerInteraction.BPI_DismissInteraction` _targetcable :!label _label_2))))

(event `/Game/BPInterfaces/BPI_PowerSystem.BPI_IsDisconnected`
  (params (Power :type Boolean))
  (bind _staticmesh (`self.StaticMesh`))
  (if Power
    (`PrimitiveComponent.SetMaterial` _staticmesh 0 "/Game/InteractiveElements/PowerGen/M_Power.M_Power")
    (goto _label)
    (else
      (`PrimitiveComponent.SetMaterial` _staticmesh 0 "/Game/InteractiveElements/PowerGen/M_Powerless.M_Powerless")
      (goto _label_2))))

(fn `UserConstructionScript`)
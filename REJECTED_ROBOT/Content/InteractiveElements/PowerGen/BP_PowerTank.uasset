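; BP_PowerTank is an interactive power tank that fills and empties visually and switches whether it generates power.
; Interaction calls play or reverse the FillingTank timeline at a configurable rate, driving a material Percentage parameter.
; It messages LinkedActor on the first filling update and when full, setting GeneratesPower, then dismisses it once fully empty.
; The construction script feeds mesh bounds into a dynamic material as BaseZ and Height.
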(event `self.ReceiveBeginPlay`
  (`TimelineComponent.SetPlayRate` (`self.FillingTank`) (`self.Filling,EmptyingRateMultiplier`)))

(event `FillTank`
  (bind _linkedactor (`self.LinkedActor`))
  (set `self.IsFilling` true)
  (bind (_direction _newtrack_0) (`Timeline|FillingTank` :!label _label)
    (:`Update`
      (bind _output_get (set `self.FillPercentage` _newtrack_0))
      (`MeshComponent.SetScalarParameterValueOnMaterials` (`self.StaticMesh`) "Percentage" _output_get)
      (`/Engine/EditorBlueprintResources/StandardMacros.DoOnce` false :!label _label_2
        (:`Completed`
          (if (`self.IsFilling`)
            (message `/Game/BPInterfaces/BPI_PlayerInteraction.BPI_CallInteraction` _linkedactor)))))
    (:`Finished`
      (if (`self.IsFilling`)
        (set `self.GeneratesPower` true)
        (message `/Game/BPInterfaces/BPI_PlayerInteraction.BPI_CallInteraction` _linkedactor)
        (else
          (set `self.GeneratesPower` false)
          (message `/Game/BPInterfaces/BPI_PlayerInteraction.BPI_DismissInteraction` _linkedactor)
          (goto _label_2 :!via `Reset`))))))

(event `EmptyTank`
  (set `self.IsFilling` false)
  (goto _label :!via `Reverse`))

(event `/Game/BPInterfaces/BPI_PlayerInteraction.BPI_CallInteraction`
  (`self.FillTank`)
  (set `self.FillPercentage` 0.0))

(event `/Game/BPInterfaces/BPI_PlayerInteraction.BPI_DismissInteraction`
  (`self.EmptyTank`)
  (set `self.FillPercentage` (`self.FillPercentage`)))

(fn `UserConstructionScript`
  (bind _dynamicmaterial (`self.DynamicMaterial`))
  (bind (_min _max) (`StaticMeshComponent.GetLocalBounds` (`self.StaticMesh`)))
  (bind _returnvalue (`PrimitiveComponent.CreateDynamicMaterialInstance` (`self.StaticMesh`) 0 null "None"))
  (set `self.DynamicMaterial` _returnvalue)
  (bind _output_get (set `self.BaseZ` (.z _min)))
  (bind _output_get_2 (set `self.Height` (- (.z _min) (.z _max))))
  (`MaterialInstanceDynamic.SetScalarParameterValue` _dynamicmaterial "BaseZ" _output_get)
  (`MaterialInstanceDynamic.SetScalarParameterValue` _dynamicmaterial "Height" (`KismetMathLibrary.Abs` _output_get_2)))
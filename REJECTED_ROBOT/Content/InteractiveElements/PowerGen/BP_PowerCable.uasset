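; Power cable actor that visually fills with power along a spline and relays an interaction to its linked actor.
; Construction builds two spline meshes per segment, giving one a colored dynamic material.
; Interaction toggles filling or draining, with Tick updating each segment's Percentage parameter from the powered distance.
; The linked actor activates when distance reaches half the spline length and is dismissed once draining begins.
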(event `self.ReceiveTick`
  (params (DeltaSeconds :type "Float (single-precision)"))
  (bind _returnvalue (* (`SplineComponent.GetSplineLength` (`self.Spline`)) 0.5))
  (if (`self.IsWorking`)
    (bind _output_get (set `self.Distance` (`KismetMathLibrary.FClamp` (+ (* (`self.FillSpeed`) DeltaSeconds) (`self.Distance`)) 0.0 _returnvalue)))
    (if (and (>= _output_get _returnvalue) (not (`self.IsPowered`)))
      (message `/Game/BPInterfaces/BPI_PlayerInteraction.BPI_CallInteraction` (`self.LinkedActor`))
      (set `self.IsPowered` true))
    (else
      (set `self.Distance` (`KismetMathLibrary.FClamp` (- (`self.Distance`) (* (`self.FillSpeed`) DeltaSeconds)) 0.0 _returnvalue))
      (if (`self.IsPowered`)
        (message `/Game/BPInterfaces/BPI_PlayerInteraction.BPI_DismissInteraction` (`self.LinkedActor`))
        (set `self.IsPowered` false))))
  (`self.PowerCable`))

(event `PowerCable`
  (bind _spline (`self.Spline`))
  (bind _returnvalue (`SplineComponent.GetDistanceAlongSplineAtSplinePoint` (`self.Spline`) (- (`self.CurrentIndex`) 1)))
  (bind _returnvalue_2 (`PrimitiveComponent.GetMaterial` (`|GetArrayItem` (`self.Components`) (- (`self.CurrentIndex`) 1)) 0))
  (for _index (range 1 (`SplineComponent.GetNumberOfSplinePoints` _spline))
    (set `self.CurrentIndex` _index)
    (if (< (`SplineComponent.GetDistanceAlongSplineAtSplinePoint` _spline (`self.CurrentIndex`)) (`self.Distance`))
      (bind _asmaterial_instance_dynamic (cast `MaterialInstanceDynamic` _returnvalue_2))
      (`MaterialInstanceDynamic.SetScalarParameterValue` _asmaterial_instance_dynamic "Percentage" -1.0)
      (else
        (bind _asmaterial_instance_dynamic_2 (cast `MaterialInstanceDynamic` _returnvalue_2))
        (`MaterialInstanceDynamic.SetScalarParameterValue` _asmaterial_instance_dynamic_2 "Percentage" (`KismetMathLibrary.FClamp` (* (- (* (/ (- (`self.Distance`) (* _returnvalue 0.5)) (- (`SplineComponent.GetDistanceAlongSplineAtSplinePoint` (`self.Spline`) (`self.CurrentIndex`)) _returnvalue)) 2.0) 1.0) -1.0) -1.0))))))

(event `/Game/BPInterfaces/BPI_PlayerInteraction.BPI_CallInteraction`
  (set `self.IsWorking` true))

(event `/Game/BPInterfaces/BPI_PlayerInteraction.BPI_DismissInteraction`
  (set `self.IsWorking` false))

(fn `UserConstructionScript`
  (bind _spline (`self.Spline`))
  (for _index (range (+ (- (`SplineComponent.GetNumberOfSplinePoints` (`self.Spline`)) 2) 1))
    (bind _returnvalue (`AddComponent|NODE_AddSplineMeshComponent-0`))
    (`PrimitiveComponent.SetCollisionEnabled` _returnvalue "NoCollision")
    (bind _returnvalue_2 (`KismetMaterialLibrary.CreateDynamicMaterialInstance` "/Game/InteractiveElements/PowerGen/M_CableMat.M_CableMat"))
    (`MaterialInstanceDynamic.SetVectorParameterValue` _returnvalue_2 "PowerOn" (`self.Color`))
    (`PrimitiveComponent.SetMaterial` _returnvalue 0 _returnvalue_2)
    (`KismetArrayLibrary.Array_Add` (`self.Components`) _returnvalue)
    (`SceneComponent.K2_AttachToComponent` _returnvalue (`self.DefaultSceneRoot`) "None" "KeepRelative" "KeepRelative" "KeepRelative" true)
    (bind (_location _tangent) (`SplineComponent.GetLocationAndTangentAtSplinePoint` _spline _index "Local"))
    (bind (_location_2 _tangent_2) (`SplineComponent.GetLocationAndTangentAtSplinePoint` _spline (+ _index 1) "Local"))
    (`SplineMeshComponent.SetStartAndEnd` _returnvalue _location _tangent _location_2 _tangent_2 true)
    (bind _returnvalue_3 (`AddComponent|NODE_AddSplineMeshComponent-1`))
    (`SceneComponent.K2_AttachToComponent` _returnvalue_3 (`self.DefaultSceneRoot`) "None" "KeepRelative" "KeepRelative" "KeepRelative" true)
    (`SplineMeshComponent.SetStartAndEnd` _returnvalue_3 _location _tangent _location_2 _tangent_2 true)))
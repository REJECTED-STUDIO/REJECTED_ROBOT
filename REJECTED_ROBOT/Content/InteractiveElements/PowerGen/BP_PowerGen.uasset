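; Movable power generator that the player grabs at handle sides to push, pull or rotate, powered by day and unpowered at night.
; Construction script sets four side meshes; box overlaps enable input at handles, and E toggles grab.
; W/S and A/D drive move and rotate timelines with the player attached, gated by line and box traces.
; End-piece spheres send interface connect messages while powered, and disconnect when overlap ends.
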(event OnComponentEndOverlap(Box0)
  (params (OverlappedComponent :type Primitive%20Component%20Object%20Reference) (OtherActor :type Actor%20Object%20Reference) (OtherComp :type Primitive%20Component%20Object%20Reference) (OtherBodyIndex :type Integer))
  (if (== (Utilities|Select :Index (Variables|Default|GetOverlappedBox) :Option%200 OtherActor :Option%201 (stale OnComponentEndOverlap(Box1) OtherActor) :Option%202 (stale OnComponentEndOverlap(Box2) OtherActor) :Option%203 (stale OnComponentEndOverlap(Box3) OtherActor)) (Game|GetPlayerCharacter 0))
    (Input|DisableInput (Game|GetPlayerController 0))
    (Variables|Default|SetGrabbed false)
    (CallFunction|StopPush)
    (Variables|Default|SetPressedW false)
    (Variables|Default|SetPressedS false)))

(event OnComponentBeginOverlap(Box0)
  (params (OverlappedComponent :type Primitive%20Component%20Object%20Reference) (OtherActor :type Actor%20Object%20Reference) (OtherComp :type Primitive%20Component%20Object%20Reference) (OtherBodyIndex :type Integer) (bFromSweep :type Boolean) (SweepResult :type Hit%20Result%20Structure%20%28by%20ref%29))
  (bind _returnvalue (Game|GetPlayerController 0))
  (Variables|Default|SetOverlappedBox 0)
  (if (== (Utilities|Select :Index (Variables|Default|GetOverlappedBox) :Option%200 OtherActor :Option%201 (stale OnComponentBeginOverlap(Box1) OtherActor) :Option%202 (stale OnComponentBeginOverlap(Box2) OtherActor) :Option%203 (stale OnComponentBeginOverlap(Box3) OtherActor)) (Game|GetPlayerCharacter 0))
    (if (or (== (Utilities|Select :Index (Variables|Default|GetOverlappedBox) :Option%200 (Variables|Default|GetTargetSM2) :Option%201 (Variables|Default|GetTargetSM3) :Option%202 (Variables|Default|GetTargetSM4) :Option%203 (Variables|Default|GetTargetSM1)) "/Game/InteractiveElements/PowerGen/SM/SM_Chwyt.SM_Chwyt") (== (Utilities|Select :Index (Variables|Default|GetOverlappedBox) :Option%200 (Variables|Default|GetTargetSM2) :Option%201 (Variables|Default|GetTargetSM3) :Option%202 (Variables|Default|GetTargetSM4) :Option%203 (Variables|Default|GetTargetSM1)) "/Game/InteractiveElements/PowerGen/SM/SM_ChwytKonc.SM_ChwytKonc"))
      (Input|EnableInput _returnvalue)
      (else
        (Input|DisableInput _returnvalue)))))

(event OnComponentBeginOverlap(Sphere2)
  (params (OverlappedComponent :type Primitive%20Component%20Object%20Reference) (OtherActor :type Actor%20Object%20Reference) (OtherComp :type Primitive%20Component%20Object%20Reference) (OtherBodyIndex :type Integer) (bFromSweep :type Boolean) (SweepResult :type Hit%20Result%20Structure%20%28by%20ref%29))
  (bind _sm_2 (Variables|Default|GetSM_2))
  (bind _staticmesh (Variables|/Script/Engine.StaticMeshComponent|GetStaticMesh _sm_2))
  (if (and (or (== _staticmesh "/Game/InteractiveElements/PowerGen/SM/SM_Konc.SM_Konc") (== _staticmesh "/Game/InteractiveElements/PowerGen/SM/SM_ChwytKonc.SM_ChwytKonc")) (Variables|Default|GetGeneratesPower))
    (Class|BPIPowerSystem|BPIIsConnected(Message) OtherActor true)
    (Variables|Default|SetConnectedActor OtherActor)))

(event OnComponentBeginOverlap(Sphere3)
  (params (OverlappedComponent :type Primitive%20Component%20Object%20Reference) (OtherActor :type Actor%20Object%20Reference) (OtherComp :type Primitive%20Component%20Object%20Reference) (OtherBodyIndex :type Integer) (bFromSweep :type Boolean) (SweepResult :type Hit%20Result%20Structure%20%28by%20ref%29))
  (if (and (or (== (Variables|/Script/Engine.StaticMeshComponent|GetStaticMesh (Variables|Default|GetSM_4)) "/Game/InteractiveElements/PowerGen/SM/SM_Konc.SM_Konc") (== 0 "/Game/InteractiveElements/PowerGen/SM/SM_ChwytKonc.SM_ChwytKonc")) (Variables|Default|GetGeneratesPower))
    (Class|BPIPowerSystem|BPIIsConnected(Message) OtherActor true)
    (Variables|Default|SetConnectedActor OtherActor)))

(event OnComponentEndOverlap(Sphere0)
  (params (OverlappedComponent :type Primitive%20Component%20Object%20Reference) (OtherActor :type Actor%20Object%20Reference) (OtherComp :type Primitive%20Component%20Object%20Reference) (OtherBodyIndex :type Integer))
  (Class|BPIPowerSystem|BPIIsDisconnected(Message) OtherActor false))

(event OnComponentEndOverlap(Sphere1)
  (params (OverlappedComponent :type Primitive%20Component%20Object%20Reference) (OtherActor :type Actor%20Object%20Reference) (OtherComp :type Primitive%20Component%20Object%20Reference) (OtherBodyIndex :type Integer))
  (Class|BPIPowerSystem|BPIIsDisconnected(Message) OtherActor false))

(event OnComponentEndOverlap(Sphere2)
  (params (OverlappedComponent :type Primitive%20Component%20Object%20Reference) (OtherActor :type Actor%20Object%20Reference) (OtherComp :type Primitive%20Component%20Object%20Reference) (OtherBodyIndex :type Integer))
  (Class|BPIPowerSystem|BPIIsDisconnected(Message) OtherActor false))

(event OnComponentEndOverlap(Sphere3)
  (params (OverlappedComponent :type Primitive%20Component%20Object%20Reference) (OtherActor :type Actor%20Object%20Reference) (OtherComp :type Primitive%20Component%20Object%20Reference) (OtherBodyIndex :type Integer))
  (Class|BPIPowerSystem|BPIIsDisconnected(Message) OtherActor false))

(event OnComponentEndOverlap(Box1)
  (params (OverlappedComponent :type Primitive%20Component%20Object%20Reference) (OtherActor :type Actor%20Object%20Reference) (OtherComp :type Primitive%20Component%20Object%20Reference) (OtherBodyIndex :type Integer))
  (if (== (Utilities|Select :Index (Variables|Default|GetOverlappedBox) :Option%200 (stale OnComponentEndOverlap(Box0) OtherActor) :Option%201 OtherActor :Option%202 (stale OnComponentEndOverlap(Box2) OtherActor) :Option%203 (stale OnComponentEndOverlap(Box3) OtherActor)) (Game|GetPlayerCharacter 0))
    (Input|DisableInput (Game|GetPlayerController 0))
    (Variables|Default|SetGrabbed false)
    (CallFunction|StopPush)
    (Variables|Default|SetPressedW false)
    (Variables|Default|SetPressedS false)))

(event OnComponentBeginOverlap(Box1)
  (params (OverlappedComponent :type Primitive%20Component%20Object%20Reference) (OtherActor :type Actor%20Object%20Reference) (OtherComp :type Primitive%20Component%20Object%20Reference) (OtherBodyIndex :type Integer) (bFromSweep :type Boolean) (SweepResult :type Hit%20Result%20Structure%20%28by%20ref%29))
  (bind _returnvalue (Game|GetPlayerController 0))
  (Variables|Default|SetOverlappedBox 1)
  (if (== (Utilities|Select :Index (Variables|Default|GetOverlappedBox) :Option%200 (stale OnComponentBeginOverlap(Box0) OtherActor) :Option%201 OtherActor :Option%202 (stale OnComponentBeginOverlap(Box2) OtherActor) :Option%203 (stale OnComponentBeginOverlap(Box3) OtherActor)) (Game|GetPlayerCharacter 0))
    (if (or (== (Utilities|Select :Index (Variables|Default|GetOverlappedBox) :Option%200 (Variables|Default|GetTargetSM2) :Option%201 (Variables|Default|GetTargetSM3) :Option%202 (Variables|Default|GetTargetSM4) :Option%203 (Variables|Default|GetTargetSM1)) "/Game/InteractiveElements/PowerGen/SM/SM_Chwyt.SM_Chwyt") (== (Utilities|Select :Index (Variables|Default|GetOverlappedBox) :Option%200 (Variables|Default|GetTargetSM2) :Option%201 (Variables|Default|GetTargetSM3) :Option%202 (Variables|Default|GetTargetSM4) :Option%203 (Variables|Default|GetTargetSM1)) "/Game/InteractiveElements/PowerGen/SM/SM_ChwytKonc.SM_ChwytKonc"))
      (Input|EnableInput _returnvalue)
      (else
        (Input|DisableInput _returnvalue)))))

(event OnComponentBeginOverlap(Sphere0)
  (params (OverlappedComponent :type Primitive%20Component%20Object%20Reference) (OtherActor :type Actor%20Object%20Reference) (OtherComp :type Primitive%20Component%20Object%20Reference) (OtherBodyIndex :type Integer) (bFromSweep :type Boolean) (SweepResult :type Hit%20Result%20Structure%20%28by%20ref%29))
  (bind _sm_1 (Variables|Default|GetSM_1))
  (bind _staticmesh (Variables|/Script/Engine.StaticMeshComponent|GetStaticMesh _sm_1))
  (if (and (or (== _staticmesh "/Game/InteractiveElements/PowerGen/SM/SM_Konc.SM_Konc") (== _staticmesh "/Game/InteractiveElements/PowerGen/SM/SM_ChwytKonc.SM_ChwytKonc")) (Variables|Default|GetGeneratesPower))
    (Class|BPIPowerSystem|BPIIsConnected(Message) OtherActor true)
    (Variables|Default|SetConnectedActor OtherActor)))

(event OnComponentBeginOverlap(Sphere1)
  (params (OverlappedComponent :type Primitive%20Component%20Object%20Reference) (OtherActor :type Actor%20Object%20Reference) (OtherComp :type Primitive%20Component%20Object%20Reference) (OtherBodyIndex :type Integer) (bFromSweep :type Boolean) (SweepResult :type Hit%20Result%20Structure%20%28by%20ref%29))
  (bind _sm_3 (Variables|Default|GetSM_3))
  (bind _staticmesh (Variables|/Script/Engine.StaticMeshComponent|GetStaticMesh _sm_3))
  (if (and (or (== _staticmesh "/Game/InteractiveElements/PowerGen/SM/SM_Konc.SM_Konc") (== _staticmesh "/Game/InteractiveElements/PowerGen/SM/SM_ChwytKonc.SM_ChwytKonc")) (Variables|Default|GetGeneratesPower))
    (Class|BPIPowerSystem|BPIIsConnected(Message) OtherActor true)
    (Variables|Default|SetConnectedActor OtherActor)))

(event OnComponentBeginOverlap(Box2)
  (params (OverlappedComponent :type Primitive%20Component%20Object%20Reference) (OtherActor :type Actor%20Object%20Reference) (OtherComp :type Primitive%20Component%20Object%20Reference) (OtherBodyIndex :type Integer) (bFromSweep :type Boolean) (SweepResult :type Hit%20Result%20Structure%20%28by%20ref%29))
  (bind _returnvalue (Game|GetPlayerController 0))
  (Variables|Default|SetOverlappedBox 2)
  (if (== (Utilities|Select :Index (Variables|Default|GetOverlappedBox) :Option%200 (stale OnComponentBeginOverlap(Box0) OtherActor) :Option%201 (stale OnComponentBeginOverlap(Box1) OtherActor) :Option%202 OtherActor :Option%203 (stale OnComponentBeginOverlap(Box3) OtherActor)) (Game|GetPlayerCharacter 0))
    (if (or (== (Utilities|Select :Index (Variables|Default|GetOverlappedBox) :Option%200 (Variables|Default|GetTargetSM2) :Option%201 (Variables|Default|GetTargetSM3) :Option%202 (Variables|Default|GetTargetSM4) :Option%203 (Variables|Default|GetTargetSM1)) "/Game/InteractiveElements/PowerGen/SM/SM_Chwyt.SM_Chwyt") (== (Utilities|Select :Index (Variables|Default|GetOverlappedBox) :Option%200 (Variables|Default|GetTargetSM2) :Option%201 (Variables|Default|GetTargetSM3) :Option%202 (Variables|Default|GetTargetSM4) :Option%203 (Variables|Default|GetTargetSM1)) "/Game/InteractiveElements/PowerGen/SM/SM_ChwytKonc.SM_ChwytKonc"))
      (Input|EnableInput _returnvalue)
      (else
        (Input|DisableInput _returnvalue)))))

(event OnComponentBeginOverlap(Box3)
  (params (OverlappedComponent :type Primitive%20Component%20Object%20Reference) (OtherActor :type Actor%20Object%20Reference) (OtherComp :type Primitive%20Component%20Object%20Reference) (OtherBodyIndex :type Integer) (bFromSweep :type Boolean) (SweepResult :type Hit%20Result%20Structure%20%28by%20ref%29))
  (bind _returnvalue (Game|GetPlayerController 0))
  (Variables|Default|SetOverlappedBox 3)
  (if (== (Utilities|Select :Index (Variables|Default|GetOverlappedBox) :Option%200 (stale OnComponentBeginOverlap(Box0) OtherActor) :Option%201 (stale OnComponentBeginOverlap(Box1) OtherActor) :Option%202 (stale OnComponentBeginOverlap(Box2) OtherActor) :Option%203 OtherActor) (Game|GetPlayerCharacter 0))
    (if (or (== (Utilities|Select :Index (Variables|Default|GetOverlappedBox) :Option%200 (Variables|Default|GetTargetSM2) :Option%201 (Variables|Default|GetTargetSM3) :Option%202 (Variables|Default|GetTargetSM4) :Option%203 (Variables|Default|GetTargetSM1)) "/Game/InteractiveElements/PowerGen/SM/SM_Chwyt.SM_Chwyt") (== (Utilities|Select :Index (Variables|Default|GetOverlappedBox) :Option%200 (Variables|Default|GetTargetSM2) :Option%201 (Variables|Default|GetTargetSM3) :Option%202 (Variables|Default|GetTargetSM4) :Option%203 (Variables|Default|GetTargetSM1)) "/Game/InteractiveElements/PowerGen/SM/SM_ChwytKonc.SM_ChwytKonc"))
      (Input|EnableInput _returnvalue)
      (else
        (Input|DisableInput _returnvalue)))))

(event OnComponentEndOverlap(Box2)
  (params (OverlappedComponent :type Primitive%20Component%20Object%20Reference) (OtherActor :type Actor%20Object%20Reference) (OtherComp :type Primitive%20Component%20Object%20Reference) (OtherBodyIndex :type Integer))
  (if (== (Utilities|Select :Index (Variables|Default|GetOverlappedBox) :Option%200 (stale OnComponentEndOverlap(Box0) OtherActor) :Option%201 (stale OnComponentEndOverlap(Box1) OtherActor) :Option%202 OtherActor :Option%203 (stale OnComponentEndOverlap(Box3) OtherActor)) (Game|GetPlayerCharacter 0))
    (Input|DisableInput (Game|GetPlayerController 0))
    (Variables|Default|SetGrabbed false)
    (CallFunction|StopPush)
    (Variables|Default|SetPressedW false)
    (Variables|Default|SetPressedS false)))

(event OnComponentEndOverlap(Box3)
  (params (OverlappedComponent :type Primitive%20Component%20Object%20Reference) (OtherActor :type Actor%20Object%20Reference) (OtherComp :type Primitive%20Component%20Object%20Reference) (OtherBodyIndex :type Integer))
  (if (== (Utilities|Select :Index (Variables|Default|GetOverlappedBox) :Option%200 (stale OnComponentEndOverlap(Box0) OtherActor) :Option%201 (stale OnComponentEndOverlap(Box1) OtherActor) :Option%202 (stale OnComponentEndOverlap(Box2) OtherActor) :Option%203 OtherActor) (Game|GetPlayerCharacter 0))
    (Input|DisableInput (Game|GetPlayerController 0))
    (Variables|Default|SetGrabbed false)
    (CallFunction|StopPush)
    (Variables|Default|SetPressedW false)
    (Variables|Default|SetPressedS false)))

(event Custom|CanPush
  (bind _returnvalue (Game|GetPlayerCharacter 0))
  (bind _canbepushed (CallFunction|FCanPush))
  (if _canbepushed
    (Pawn|Components|CharacterMovement|DisableMovement (Variables|/Script/Engine.Character|GetCharacterMovement _returnvalue))
    (Transformation|AttachActorToActor _returnvalue self "None" "KeepWorld" "KeepWorld" "KeepWorld" true)
    (switch int (Variables|Default|GetForward/Backwards)
      (:1
        (CallFunction|Push :!label _label))
      (:2
        (goto _label))
      (:3
        (CallFunction|Rotate :!label _label_2))
      (:4
        (goto _label_2)))))

(event Custom|Push
  ;[0.1771 0.1771 0.1771] Pchanie/Ciagniecie
  (Utilities|FlowControl|Sequence
    (:then_0
      (Variables|Default|SetCurrentLocation (Transformation|GetActorLocation))
      (bind _position (Timeline|PushTimeline PlayFromStart)
        (:Update
          (Transformation|SetActorRelativeLocation (+ (* _position (Variables|Default|GetPushDirection) (Utilities|Select :Index (Variables|Default|GetForward/Backwards) :Option%200 0.0 :Option%201 1e+02 :Option%202 -1e+02)) (Variables|Default|GetCurrentLocation))))
        (:Finished
          (if (or (Variables|Default|GetPressedW) (Variables|Default|GetPressedS))
            (CallFunction|CanPush)
            (else
              (CallFunction|StopPush))))))
    (:then_1
      (Utilities|Time|SetTimerbyEvent (delegate Custom|CheckIfCanPush) 0.2 true))))

(event Custom|StopRotate
  ;[0.1771 0.1771 0.1771] Pchanie/Ciagniecie
  (Audio|Components|Audio|Stop (Variables|Default|GetRotateTimeline)))

(event Custom|Rotate
  ;[0.1771 0.1771 0.1771] Pchanie/Ciagniecie
  (Variables|Default|SetCurrentRotation (Variables|Default|GetCurrentRotation))
  (Utilities|FlowControl|Sequence
    (:then_0
      (if (Variables|Default|GetPressedA)
        (bind _position (Timeline|RotateTimeline Play)
          (:Update
            (Transformation|SetActorRelativeRotation (Math|Rotator|MakeRotator 0.0 0.0 (+ (* _position 3.6e+02) (.Yaw (Math|Rotator|BreakRotator (Variables|Default|GetCurrentRotation)))))))
          (:Finished
            (if (Variables|Default|GetPressedA)
              (CallFunction|Rotate)
              (Variables|Default|SetNew%20Time 0.0)
              (Timeline|RotateTimeline SetNewTime)
              (elif (Variables|Default|GetPressedD)
                (CallFunction|Rotate)
                (Variables|Default|SetNew%20Time 5.0)
                (Timeline|RotateTimeline SetNewTime)
                (else
                  (CallFunction|StopRotate))))))))
    (:then_1
      (if (Variables|Default|GetPressedD)
        (Timeline|RotateTimeline Reverse)))))

(event Custom|StopPush
  ;[0.1771 0.1771 0.1771] Pchanie/Ciagniecie
  (Audio|Components|Audio|Stop (Variables|Default|GetPushTimeline)))

(event Custom|CheckIfCanPush
  ;[0.1771 0.1771 0.1771] Pchanie/Ciagniecie
  (bind _canbepushed (CallFunction|FCanPush))
  (if (not _canbepushed)
    (CallFunction|StopPush)))

(event Custom|UpdatePowerLogic
  (bind _staticmesh (Variables|Default|GetStaticMesh))
  (if (Variables|Default|GetGeneratesPower)
    (Rendering|Material|SetMaterial _staticmesh 0 "/Game/InteractiveElements/PowerGen/M_Power.M_Power")
    (else
      (Rendering|Material|SetMaterial _staticmesh 0 "/Game/InteractiveElements/PowerGen/M_Powerless.M_Powerless"))))

(event EventBPINotifyDay
  (Variables|Default|SetGeneratesPower true)
  (CallFunction|UpdatePowerLogic))

(event EventBPINotifyNight
  (Variables|Default|SetGeneratesPower false)
  (CallFunction|UpdatePowerLogic))

(event Input|KeyboardEvents|DebugKeyA
  (params (Key :type Key%20Structure :default "None") (ActionValue :type Input%20Action%20Value%20Structure))
  (:Pressed
    (if (not (Variables|Default|GetPressedD))
      (if (Variables|Default|GetCanRotate)
        (if (Variables|Default|GetGrabbed)
          (Variables|Default|SetPressedA true)
          (Variables|Default|SetCanPushBool false)
          (Variables|Default|SetForward/Backwards 3)
          (if (Variables|Default|GetPressedD)
            (CallFunction|StopRotate)
            (elif (Variables|Default|GetGrabbed)
              (Variables|Default|SetPushDirection (Transformation|GetActorForwardVector (Game|GetPlayerCharacter 0)))
              (CallFunction|CanPush)))))))
  (:Released
    (Variables|Default|SetPressedA false)
    (if (not (Variables|Default|GetPressedD))
      (CallFunction|StopRotate)
      (Variables|Default|SetCanPushBool true))))

(event Input|KeyboardEvents|DebugKeyD
  (params (Key :type Key%20Structure :default "None") (ActionValue :type Input%20Action%20Value%20Structure))
  (:Pressed
    (if (not (Variables|Default|GetPressedA))
      (if (Variables|Default|GetCanRotate)
        (if (Variables|Default|GetGrabbed)
          (Variables|Default|SetPressedD true)
          (Variables|Default|SetCanPushBool false)
          (Variables|Default|SetForward/Backwards 4)
          (if (Variables|Default|GetPressedA)
            (CallFunction|StopRotate)
            (elif (Variables|Default|GetGrabbed)
              (Variables|Default|SetPushDirection (Transformation|GetActorForwardVector (Game|GetPlayerCharacter 0)))
              (CallFunction|CanPush)))))))
  (:Released
    (Variables|Default|SetPressedD false)
    (if (not (Variables|Default|GetPressedA))
      (CallFunction|StopRotate)
      (Variables|Default|SetCanPushBool true))))

(event Input|KeyboardEvents|DebugKeyE
  (params (Key :type Key%20Structure :default "None") (ActionValue :type Input%20Action%20Value%20Structure))
  (bind _returnvalue (Game|GetPlayerCharacter 0))
  (bind _overlappedbox (Variables|Default|GetOverlappedBox))
  (bind _arrow (Variables|Default|GetArrow))
  (bind _arrow2 (Variables|Default|GetArrow2))
  (bind _arrow3 (Variables|Default|GetArrow3))
  (bind _arrow1 (Variables|Default|GetArrow1))
  (bind _returnvalue_2 (Utilities|Select :Index _overlappedbox :Option%200 _arrow2 :Option%201 _arrow :Option%202 _arrow3 :Option%203 _arrow1))
  (:Pressed
    (Utilities|FlowControl|FlipFlop
      (:A
        (Variables|Default|SetGrabbed true)
        (Transformation|SetActorLocationAndRotation (Game|GetPlayerCharacter 0) (Transformation|GetWorldLocation _returnvalue_2) (Transformation|GetWorldRotation _returnvalue_2))
        (Pawn|Components|CharacterMovement|SetMovementMode (Variables|/Script/Engine.Character|GetCharacterMovement (Game|GetPlayerCharacter 0)) "MOVE_None" 0))
      (:B
        (Variables|Default|SetGrabbed false)
        (Variables|Default|SetPressedW false)
        (Variables|Default|SetPressedS false)
        (Pawn|Components|CharacterMovement|SetMovementMode (Variables|/Script/Engine.Character|GetCharacterMovement _returnvalue) "MOVE_Walking" 0)
        (Transformation|DetachFromActor _returnvalue "KeepWorld" "KeepWorld" "KeepWorld")))))

(event Input|KeyboardEvents|DebugKeyW
  (params (Key :type Key%20Structure :default "None") (ActionValue :type Input%20Action%20Value%20Structure))
  (:Pressed
    (if (not (Variables|Default|GetPressedS))
      (if (Variables|Default|GetCanPushBool)
        (if (Variables|Default|GetGrabbed)
          (Variables|Default|SetPressedW true)
          (Variables|Default|SetForward/Backwards 1)
          (Variables|Default|SetCanRotate false)
          (if (Variables|Default|GetPressedS)
            (CallFunction|StopPush)
            (elif (Variables|Default|GetGrabbed)
              (Variables|Default|SetPushDirection (Transformation|GetActorForwardVector (Game|GetPlayerCharacter 0)))
              (CallFunction|CanPush)))))))
  (:Released
    (Variables|Default|SetPressedW false)
    (if (not (Variables|Default|GetPressedS))
      (CallFunction|StopPush)
      (Variables|Default|SetCanRotate true))))

(event Input|KeyboardEvents|DebugKeyS
  (params (Key :type Key%20Structure :default "None") (ActionValue :type Input%20Action%20Value%20Structure))
  (:Pressed
    (if (not (Variables|Default|GetPressedW))
      (if (Variables|Default|GetCanPushBool)
        (if (Variables|Default|GetGrabbed)
          (Variables|Default|SetPressedS true)
          (Variables|Default|SetForward/Backwards 2)
          (Variables|Default|SetCanRotate false)
          (if (Variables|Default|GetPressedW)
            (CallFunction|StopPush)
            (elif (Variables|Default|GetGrabbed)
              (Variables|Default|SetPushDirection (Transformation|GetActorForwardVector (Game|GetPlayerCharacter 0)))
              (CallFunction|CanPush)))))))
  (:Released
    (Variables|Default|SetPressedS false)
    (if (not (Variables|Default|GetPressedW))
      (CallFunction|StopPush)
      (Variables|Default|SetCanRotate true))))

(fn ConstructionScript
  (Utilities|FlowControl|Sequence
    (:then_0
      (Components|StaticMesh|SetStaticMesh (Variables|Default|GetSM_1) (Variables|Default|GetTargetSM1)))
    (:then_1
      (Components|StaticMesh|SetStaticMesh (Variables|Default|GetSM_3) (Variables|Default|GetTargetSM3)))
    (:then_2
      (Components|StaticMesh|SetStaticMesh (Variables|Default|GetSM_2) (Variables|Default|GetTargetSM2)))
    (:then_3
      (Components|StaticMesh|SetStaticMesh (Variables|Default|GetSM_4) (Variables|Default|GetTargetSM4)))))

(fn FCanPush
  (bind _returnvalue (Game|GetPlayerCharacter 0))
  (bind _returnvalue_2 (Transformation|GetActorLocation))
  (bind _staticmesh (Variables|Default|GetStaticMesh))
  (bind _returnvalue_3 (Transformation|GetActorLocation _returnvalue))
  (bind (_outhit _returnvalue_4) (Collision|LineTraceByChannel _returnvalue_3 (+ _returnvalue_3 (* (Transformation|GetActorForwardVector _returnvalue) 1e+02)) "TraceTypeQuery1" false (Utilities|Array|MakeArray _returnvalue) "None" false))
  (if _returnvalue_4
    (if (== (.HitActor (Collision|BreakHitResult _outhit)) self)
      (bind _returnvalue_5 (Collision|BoxTraceByChannel (+ _returnvalue_2 "0.000000,0.000000,50.000000") (+ (+ _returnvalue_2 (* (Variables|Default|GetPushDirection) (Utilities|Select :Index (Variables|Default|GetForward/Backwards) :Option%200 0.0 :Option%201 1e+02 :Option%202 -1e+02)) "0.000000,0.000000,50.000000") "0.000000,10.000000,0.000000") (* (.boxextent (StaticMesh|GetBounds (Variables|/Script/Engine.StaticMeshComponent|GetStaticMesh _staticmesh))) (Variables|/Script/Engine.SceneComponent|GetRelativeScale3D _staticmesh)) "0, 0, 0" "TraceTypeQuery1" false 0 "ForDuration"))
      (return (not _returnvalue_5)))))
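; Checkpoint actor that registers itself with actors entering its box trigger and later serves as their respawn point.
; On overlap it sends a save-checkpoint interface message with itself to the other actor, leaving storage to that actor.
; Its load-checkpoint interface event moves the given user to the box's world location and rotation.
; The construction script toggles the static mesh's visibility when IsVisible is false.
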(event `self.Box.OnComponentBeginOverlap`
  (params (OverlappedComponent :type "PrimitiveComponent Object Reference") (OtherActor :type "Actor Object Reference") (OtherComp :type "PrimitiveComponent Object Reference") (OtherBodyIndex :type Integer) (bFromSweep :type Boolean) (SweepResult :type "HitResult Structure (by ref)"))
  (message `/Game/BPInterfaces/BPI_PlayerInteraction.BPI_SaveCheckpoint` OtherActor self))

(event `/Game/BPInterfaces/BPI_PlayerInteraction.BPI_LoadCheckpoint`
  (params (CheckpointUser :type "Actor Object Reference"))
  (bind _box (`self.Box`))
  (`self.K2_SetActorLocationAndRotation` CheckpointUser (`SceneComponent.K2_GetComponentLocation` _box) (`SceneComponent.K2_GetComponentRotation` _box) false false))

(fn `UserConstructionScript`
  (if (not (`self.IsVisible`))
    (`SceneComponent.ToggleVisibility` (`self.StaticMesh`) false)))